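; Coin pickup for the runner game that adds to the game mode's coin count and plays a sound.
; Touching the mesh collects and destroys it immediately.
; With the character's magnet active, overlapping the sphere counts it at once and sets Used to block mesh collection, while a timeline interpolates the coin toward the player with a Slide offset until its delayed destruction.
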(event `self.StaticMesh.OnComponentBeginOverlap`
  (params (OverlappedComponent :type "PrimitiveComponent Object Reference") (OtherActor :type "Actor Object Reference") (OtherComp :type "PrimitiveComponent Object Reference") (OtherBodyIndex :type Integer) (bFromSweep :type Boolean) (SweepResult :type "HitResult Structure (by ref)"))
  ;[1 1 1] Pickup without a magnet
  (cast `/Game/ThirdPersonBP/Blueprints/ThirdPersonCharacter` OtherActor)
  (bind _asthird_person_game_mode (cast `/Game/ThirdPersonBP/Blueprints/ThirdPersonGameMode` (`GameplayStatics.GetGameMode`)))
  (if (not (`self.Used`))
    (set `/Game/ThirdPersonBP/Blueprints/ThirdPersonGameMode.Coins` (+ (`/Game/ThirdPersonBP/Blueprints/ThirdPersonGameMode.Coins` _asthird_person_game_mode) 1) _asthird_person_game_mode)
    (`GameplayStatics.SpawnSound2D` "/Game/RunnerFiles/SFX/Pickup_SFX.Pickup_SFX" 1.0 1.0 0.0 null)
    (`self.K2_DestroyActor`)))

(event `self.Sphere.OnComponentBeginOverlap`
  (params (OverlappedComponent :type "PrimitiveComponent Object Reference") (OtherActor :type "Actor Object Reference") (OtherComp :type "PrimitiveComponent Object Reference") (OtherBodyIndex :type Integer) (bFromSweep :type Boolean) (SweepResult :type "HitResult Structure (by ref)"))
  ;[1 1 1] Pickup coin with magnet
  (bind _asthird_person_character (cast `/Game/ThirdPersonBP/Blueprints/ThirdPersonCharacter` OtherActor))
  (if (`/Game/ThirdPersonBP/Blueprints/ThirdPersonCharacter.Magnet_Active` _asthird_person_character)
    (`|ExecutionSequence`
      (:`then_0`
        (bind _asthird_person_game_mode (cast `/Game/ThirdPersonBP/Blueprints/ThirdPersonGameMode` (`GameplayStatics.GetGameMode`)))
        (`/Engine/EditorBlueprintResources/StandardMacros.IncrementInt` (`/Game/ThirdPersonBP/Blueprints/ThirdPersonGameMode.Coins` _asthird_person_game_mode)
          (:`  `
            (set `self.Used` true)
            (`GameplayStatics.SpawnSound2D` "/Game/RunnerFiles/SFX/Pickup_SFX.Pickup_SFX" 1.0 1.0 0.0 null)
            (`KismetSystemLibrary.Delay` 1.0)
            (`self.K2_DestroyActor`))))
      (:`then_1`
        (bind (_direction _slide) (`Timeline|Timeline_0`)
          (:`Update`
            (`self.K2_SetActorLocation` (+ _slide (`KismetMathLibrary.VInterpTo` (.location (`self.GetTransform`)) (`self.K2_GetActorLocation` (`GameplayStatics.GetPlayerCharacter` 0)) (`GameplayStatics.GetWorldDeltaSeconds`) 10.0)))))))))

(fn `UserConstructionScript`)