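; Magnet pickup for the runner that temporarily switches on the player's magnet effect.
; On overlap with the ThirdPersonCharacter it sets MagnetActive, hides its mesh, and after a ten-second delay clears the flag on player 0 and destroys itself.
; The magnet behaviour itself lives outside this actor; debug strings print when the effect starts and ends.
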(event `self.ReceiveActorBeginOverlap`
  (params (OtherActor :type "Actor Object Reference"))
  ;[1 1 1] Magnet
  (bind _asthird_person_character (cast `/Game/ThirdPersonBP/Blueprints/ThirdPersonCharacter` OtherActor))
  (set `/Game/ThirdPersonBP/Blueprints/ThirdPersonCharacter.Magnet_Active` true _asthird_person_character)
  (`KismetSystemLibrary.PrintString` "MAGNET ACTIVE")
  (`SceneComponent.SetVisibility` (`self.StaticMesh`) false false)
  (`KismetSystemLibrary.Delay` 10.0)
  (bind _asthird_person_character_2 (cast `/Game/ThirdPersonBP/Blueprints/ThirdPersonCharacter` (`GameplayStatics.GetPlayerCharacter` 0)))
  (set `/Game/ThirdPersonBP/Blueprints/ThirdPersonCharacter.Magnet_Active` false _asthird_person_character_2)
  (`KismetSystemLibrary.PrintString` "MAGNET INACTIVE")
  (`self.K2_DestroyActor`))

(fn `UserConstructionScript`)